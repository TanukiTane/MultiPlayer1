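; Multiplayer game mode that balances joining players between two teams.
; On PostLogin it casts the new player to BP_MPGameController, puts it on Team 2 if that team is smaller, otherwise on Team 1, sets its TeamID and stores it in that team's array.
; A failed cast prints an error, and the logout handler is empty, so players are never removed from the arrays here.
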(event EventBeginPlay)

(event EventTick
  (params (DeltaSeconds :type Float%20%28single-precision%29)))

(event EventPostLogin
  (params (NewPlayer :type Player%20Controller%20Object%20Reference))
  (bind _asbp_mpgame_controller (Utilities|Casting|CastToBP_MPGameController NewPlayer)
    (:then
      (if (< (Utilities|Array|Length (Variables|Default|GetTeam2)) (Utilities|Array|Length (Variables|Default|GetTeam1)))
        (Default|SetTeamID _asbp_mpgame_controller 2)
        (Utilities|Array|Add (Variables|Default|GetTeam2) _asbp_mpgame_controller)
        (else
          (Default|SetTeamID _asbp_mpgame_controller 1)
          (Utilities|Array|Add (Variables|Default|GetTeam1) _asbp_mpgame_controller))))
    (:CastFailed
      (Development|PrintString "Post login error"))))

(event EventOnLogout
  (params (ExitingController :type Controller%20Object%20Reference)))

(fn ConstructionScript)