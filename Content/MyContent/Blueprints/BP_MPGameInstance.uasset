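; Game instance Blueprint that handles LAN multiplayer sessions: hosting, searching for and joining games.
; CreateGame creates a LAN session and, on success, opens Level1 as a listen server.
; GetGames prints each found server's name, player counts and ping, while JoinToGame runs its own single-result search and joins that session.
; Session failures, network errors and travel errors are only reported through printed messages.
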(event Custom|CreateGame
  (|Session (Game|GetPlayerController 0) 16 true
    (:OnSuccess
      (Game|OpenLevel(byName) "Level1" true "listen"))
    (:OnFailure
      (Development|PrintString "Error"))))

(event Custom|GetGames
  (bind _results (|FindSessions (Game|GetPlayerController 0) 5 true)
    (:OnSuccess
      (for _array_element _results
        (Development|PrintString (Utilities|String|Append "Server:" (Class|FindSessionsCallbackProxy|GetServerName _array_element) "Players" (Utilities|String|ToString(Integer) (Class|FindSessionsCallbackProxy|GetCurrentPlayers _array_element)) "/" (Utilities|String|ToString(Integer) (Class|FindSessionsCallbackProxy|GetMaxPlayers _array_element)) "Ping" (Utilities|String|ToString(Integer) (Class|FindSessionsCallbackProxy|GetPinginMs _array_element))))))
    (:OnFailure
      (Development|PrintString "Game search error"))))

(event Custom|JoinToGame
  (bind _returnvalue (Game|GetPlayerController 0))
  (bind _results (|FindSessions _returnvalue 1 true)
    (:OnSuccess
      (for _array_element _results
        (|JoinSession _returnvalue _array_element
          (:OnFailure
            (Development|PrintString "Join to game failed")))))))

(event EventHandleNetworkError
  (params (FailureType :type ENetworkFailure%20Enum :default "NetDriverAlreadyExists") (bIsServer :type Boolean))
  (Development|PrintString (Utilities|String|Append "Network Error" (Utilities|String|EnumtoString FailureType) "On server" (Utilities|String|ToString(Boolean) bIsServer))))

(event EventHandleTravelError
  (params (FailureType :type ETravelFailure%20Enum :default "NoLevel"))
  (Development|PrintString (Utilities|String|EnumtoString FailureType)))