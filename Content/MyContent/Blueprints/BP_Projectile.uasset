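; Multiplayer projectile actor that flies straight, damages BP_MPPawn targets on contact and explodes.
; The server moves it along its forward vector each Tick without sweeping and handles sphere overlaps, ignoring its owner and other projectiles.
; Any other hit triggers a multicast explosion emitter and destroys the projectile, with damage applied only to pawns.
; A timer started on BeginPlay also destroys it through a server event when its lifetime expires.
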(event OnComponentBeginOverlap(Sphere1)
  (params (OverlappedComponent :type Primitive%20Component%20Object%20Reference) (OtherActor :type Actor%20Object%20Reference) (OtherComp :type Primitive%20Component%20Object%20Reference) (OtherBodyIndex :type Integer) (bFromSweep :type Boolean) (SweepResult :type Hit%20Result%20Structure%20%28by%20ref%29))
  (if (Networking|IsServer)
    (CallFunction|ServerCollision OtherActor (Transformation|GetActorLocation))))

(event Custom|LifeEnded
  (CallFunction|ServerLifeEnded))

(event Custom|Server_LifeEnded
  (Actor|DestroyActor))

(event Custom|Server_Move
  (params (DeltaTime :type Float%20%28single-precision%29))
  (Transformation|SetActorLocation (+ (Transformation|GetActorLocation) (* (Transformation|GetActorForwardVector) (* DeltaTime (Variables|Default|GetSpeed)))) false false))

(event Custom|Server_collision
  (params (Other%20Actor :type Actor%20Object%20Reference) (Location :type Vector))
  (if (!= Other%20Actor (Components|GetOwner))
    (bind _asbp_mppawn (Utilities|Casting|CastToBP_MPPawn Other%20Actor)
      (:then
        (Default|TakeDamage _asbp_mppawn (Variables|Default|GetDamage)))
      (:CastFailed
        (Utilities|Casting|CastToBP_Projectile Other%20Actor
          (:CastFailed
            _))))
    (CallFunction|MulticastHitEffect Location)
    (CallFunction|ServerLifeEnded)))

(event Custom|SpawnHitEffect
  (params (Hit%20Location :type Vector))
  (Effects|SpawnEmitteratLocation "/Game/StarterContent/Particles/P_Explosion.P_Explosion" Hit%20Location))

(event Custom|Multicast_HitEffect
  (params (HitLocation :type Vector))
  (CallFunction|SpawnHitEffect HitLocation))

(event EventBeginPlay
  (Utilities|Time|SetTimerbyEvent (delegate Custom|LifeEnded) (Variables|Default|GetTTL)))

(event Collision|EventActorBeginOverlap
  (params (OtherActor :type Actor%20Object%20Reference)))

(event EventTick
  (params (DeltaSeconds :type Float%20%28single-precision%29))
  (if (Networking|IsServer)
    (CallFunction|ServerMove DeltaSeconds)))

(fn ConstructionScript)